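; Reactor room light rig that switches its lights on when something enters its trigger sphere and goes dark when the player loses.
; Sphere overlap makes three point lights visible and plays a Brightness timeline that drives their intensity.
; HideLights hides those lights and their three lamp components, ahead of the explosion on a loss.
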(event OnComponentBeginOverlap(Sphere)
  (params (OverlappedComponent :type Primitive%20Component%20Object%20Reference) (OtherActor :type Actor%20Object%20Reference) (OtherComp :type Primitive%20Component%20Object%20Reference) (OtherBodyIndex :type Integer) (bFromSweep :type Boolean) (SweepResult :type Hit%20Result%20Structure%20%28by%20ref%29))
  (Utilities|FlowControl|Sequence
    (:then_0
      (Rendering|SetVisibility (Variables|Default|GetPointLight1) true false))
    (:then_1
      (bind _brightness (Timeline|Brightness Play)
        (:Update
          (Rendering|Components|Light|SetIntensity (Variables|Default|GetPointLight) _brightness))))))

(event Custom|HideLights
  ;[1 1 1] Disable Lights if Player lost (Ready for Explosion)
  (Rendering|SetVisibility (Variables|Default|GetPointLight) false false))

(fn ConstructionScript)