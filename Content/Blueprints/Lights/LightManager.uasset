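; LightManager is a Blueprint that switches groups of level lights on or off in response to events.
; Three enable events each loop over their own group of outside Xmas lights and call TurnOnOutsideLights on every entry.
; A one-minute warning event calls WarningLights on each warning light in the same way.
; A separate event hides the reactor room lights through a single reference.
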(event Custom|EnableLights3
  (CallFunction|EL3))

(event Custom|1MinWarning
  (CallFunction|WL))

(event Custom|EnableLights1
  (CallFunction|EL1))

(event Custom|HideReactorLights
  (Default|HideLights (Variables|Default|GetReactorRoomLights)))

(event Custom|EnableLights2
  (CallFunction|EL2))

(fn ConstructionScript)

(fn EL1
  (for _array_element (Variables|Default|GetOutsideXmas%20Lights%20Group1)
    (Default|TurnonOutsideLights _array_element))
  (return))

(fn EL2
  (for _array_element (Variables|Default|GetOutsideXmas%20Lights%20Group2)
    (Default|TurnonOutsideLights _array_element))
  (return))

(fn EL3
  (for _array_element (Variables|Default|GetOutsideXmas%20Lights%20Group3)
    (Default|TurnonOutsideLights _array_element))
  (return))

(fn WL
  (for _array_element (Variables|Default|GetWarningLights)
    (Default|WarningLights _array_element))
  (return))