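; Interior wall light Blueprint whose point light can shift to random colours.
; ChangeColour starts a looping one-second timer bound back to itself and sets the light colour from a random unit vector.
; BeginPlay is empty and nothing in this file calls ChangeColour, so the cycle needs an external trigger.
; A disconnected branch chain that picks from a fixed colour palette is left unused.
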(event Custom|Change%20Colour
  (Utilities|Time|SetTimerbyEvent (delegate Custom|Change%20Colour) 1.0 true)
  (Rendering|Components|Light|SetLightColor (Variables|Default|GetPointLight) (Math|Conversions|ToLinearColor(Vector) (Math|Random|RandomUnitVector)) true))

(event EventBeginPlay)

(fn ConstructionScript)