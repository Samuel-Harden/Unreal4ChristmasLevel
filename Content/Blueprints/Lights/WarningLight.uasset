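; WarningLight is an alarm light prop that switches on and spins when triggered, according to its comment by ThirdPersonCharacter.
; The WarningLights event sets a rotate flag, shows four point lights and plays the warning sound, with no matching off path.
; While the flag is set, Tick yaws the Cylinder by a scaled RotationSpeed each frame, independent of delta time, so spin rate follows frame rate.
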(event Custom|WarningLights
  ;[1 1 1] Function called from ThirdPersonCharacter
  (Variables|Default|SetRotate true)
  (Rendering|SetVisibility (Variables|Default|GetPointLight4) true false)
  (Audio|Components|Audio|Play (Variables|Default|GetWarningSound) 0.0))

(event EventTick
  (params (DeltaSeconds :type Float%20%28single-precision%29))
  ;[1 1 1] Rotate the Warning Lights
  (if (Variables|Default|GetRotate)
    (Transformation|AddLocalRotation (Variables|Default|GetCylinder) (* (Math|Rotator|MakeRotator 0.0 0.0 (Variables|Default|GetRotationSpeed)) 0.1) false false)))

(fn ConstructionScript)