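; Outdoor Christmas lights Blueprint that blinks six colored bulbs once TurnOnOutsideLights is called.
; The first active Tick lights red, green and blue, so they alternate against yellow, white and pink, assuming those start off.
; Later Ticks pass through a half-second Delay, then flip each bulb between its color and an off material, tracked by per-bulb booleans.
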(event Custom|TurnOnOutsideLights
  (Variables|Default|SetChangeLights true))

(event EventTick
  (params (DeltaSeconds :type Float%20%28single-precision%29))
  (bind _redlight (Variables|Default|GetRedLight))
  (bind _yellowlight (Variables|Default|GetYellowLight))
  (bind _greenlight (Variables|Default|GetGreenLight))
  (bind _whitelight (Variables|Default|GetWhiteLight))
  (bind _bluelight (Variables|Default|GetBlueLight))
  (bind _pinklight (Variables|Default|GetPinkLight))
  (if (Variables|Default|GetChangeLights)
    (if (Variables|Default|GetInitial%20LightsSet)
      (Utilities|FlowControl|Delay 0.5)
      (if (Variables|Default|GetRedLightOn)
        (Rendering|Material|SetMaterial _redlight 0 "/Game/Blueprints/Lights/LightsOff_Material.LightsOff_Material")
        (Variables|Default|SetRedLightOn false)
        (else
          (Rendering|Material|SetMaterial _redlight 0 "/Game/Blueprints/Puzzles/BallPuzzle/RedBall.RedBall")
          (Variables|Default|SetRedLightOn true)))
      (if (Variables|Default|GetYellowLightOn)
        (Rendering|Material|SetMaterial _yellowlight 0 "/Game/Blueprints/Lights/LightsOff_Material.LightsOff_Material")
        (Variables|Default|SetYellowLightOn false)
        (else
          (Rendering|Material|SetMaterial _yellowlight 0 "/Game/Blueprints/Puzzles/BallPuzzle/YellowBall.YellowBall")
          (Variables|Default|SetYellowLightOn true)))
      (if (Variables|Default|GetGreenLightOn)
        (Rendering|Material|SetMaterial _greenlight 0 "/Game/Blueprints/Lights/LightsOff_Material.LightsOff_Material")
        (Variables|Default|SetGreenLightOn false)
        (else
          (Rendering|Material|SetMaterial _greenlight 0 "/Game/Blueprints/Puzzles/BallPuzzle/GreenBall.GreenBall")
          (Variables|Default|SetGreenLightOn true)))
      (if (Variables|Default|GetWhiteLightOn)
        (Rendering|Material|SetMaterial _whitelight 0 "/Game/Blueprints/Lights/LightsOff_Material.LightsOff_Material")
        (Variables|Default|SetWhiteLightOn false)
        (else
          (Rendering|Material|SetMaterial _whitelight 0 "/Game/Blueprints/Puzzles/BallPuzzle/WhiteBall.WhiteBall")
          (Variables|Default|SetWhiteLightOn true)))
      (if (Variables|Default|GetBlueLightOn)
        (Rendering|Material|SetMaterial _bluelight 0 "/Game/Blueprints/Lights/LightsOff_Material.LightsOff_Material")
        (Variables|Default|SetBlueLightOn false)
        (else
          (Rendering|Material|SetMaterial _bluelight 0 "/Game/Blueprints/Puzzles/BallPuzzle/BlueBall.BlueBall")
          (Variables|Default|SetBlueLightOn true)))
      (if (Variables|Default|GetPinkLightOn)
        (Rendering|Material|SetMaterial _pinklight 0 "/Game/Blueprints/Lights/LightsOff_Material.LightsOff_Material")
        (Variables|Default|SetPinkLightOn false)
        (else
          (Rendering|Material|SetMaterial _pinklight 0 "/Game/Blueprints/Puzzles/BallPuzzle/PinkBall.PinkBall")
          (Variables|Default|SetPinkLightOn true)))
      (else
        (Rendering|Material|SetMaterial (Variables|Default|GetRedLight) 0 "/Game/Blueprints/Puzzles/BallPuzzle/RedBall.RedBall")
        (Variables|Default|SetRedLightOn true)
        (Rendering|Material|SetMaterial (Variables|Default|GetGreenLight) 0 "/Game/Blueprints/Puzzles/BallPuzzle/GreenBall.GreenBall")
        (Variables|Default|SetGreenLightOn true)
        (Rendering|Material|SetMaterial (Variables|Default|GetBlueLight) 0 "/Game/Blueprints/Puzzles/BallPuzzle/BlueBall.BlueBall")
        (Variables|Default|SetBlueLightOn true)
        (Variables|Default|SetInitial%20LightsSet true)))))

(fn ConstructionScript)