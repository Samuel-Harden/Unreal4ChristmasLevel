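; TimeManager runs the game's countdown clock and triggers Game Over on the player character when time runs out before a win.
; After an initial delay for the opening cinematic, Tick uses a one-second Delay to step minutes and seconds down.
; It also fires the LightManager's one-minute warning and the character's final countdown near ten seconds.
; GameWon halts the countdown, and two debug events adjust the time.
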(event Custom|Add%20Time
  ;[1 1 1] Debugging Events
  (Variables|Default|SetMins (+ (Variables|Default|GetMins) 1)))

(event Custom|GameWon
  ;[1 1 1] Update GameWon
  (Variables|Default|SetPlayerWon true))

(event Custom|SetTimeTo15
  ;[1 1 1] Debugging Events
  (Variables|Default|SetSeconds 15)
  (Variables|Default|SetMins 0))

(event EventTick
  (params (DeltaSeconds :type Float%20%28single-precision%29))
  (bind _playerwon (Variables|Default|GetPlayerWon))
  ;[1 1 1] Event Tick + Sequence (Delay for initial game cinematic)
  (if (Variables|Default|GetInitialDelay)
    _
    (else
      (Utilities|FlowControl|Delay 12.0)
      (Variables|Default|SetInitialDelay true)))
  (if (Variables|Default|GetInitialDelay)
    (Utilities|FlowControl|Sequence
      (:then_0
        ;[1 1 1] Check if the game has been won, if not keep updating
        (if (not _playerwon)
          ;[1 1 1] Check if the game has been lost, if not keep updating
          (if (Variables|Default|GetPlayerLost)
            ;[1 1 1] No time left, Player has Lost. Call Game Over
            (bind _asthird_person_character (Utilities|Casting|CastToThirdPersonCharacter (Game|GetPlayerCharacter 0) :!label _label))
            (Default|GameOver _asthird_person_character)
            (else
              ;[1 1 1] Timer Countdown
              (Utilities|FlowControl|Delay 1.0)
              (Variables|Default|SetSeconds (- (Variables|Default|GetSeconds) 1))
              (if (< (Variables|Default|GetSeconds) 0)
                (Variables|Default|SetMins (- (Variables|Default|GetMins) 1))
                (Variables|Default|SetSeconds 59))
              (if (== (Variables|Default|GetSeconds) 0)
                (if (== (Variables|Default|GetMins) 0)
                  (Variables|Default|SetPlayerLost true)))))))
      (:then_1
        (if (not _playerwon)
          (if (Variables|Default|GetPlayerLost)
            (goto _label)
            (else
              ;[1 1 1] Call ThirdPersonCharacter, starting 1min Warning Lights
              (if (== (Variables|Default|GetSeconds) 0)
                (if (== (Variables|Default|GetMins) 1)
                  (Default|1MinWarning (Variables|Default|GetLightManager))))))))
      (:then_2
        (if (== (Variables|Default|GetSeconds) 11)
          (if (== (Variables|Default|GetMins) 0)
            (bind _asthird_person_character_2 (Utilities|Casting|CastToThirdPersonCharacter (Game|GetPlayerCharacter 0)))
            (Default|10SecCountdown _asthird_person_character_2)))))))

(fn ConstructionScript)