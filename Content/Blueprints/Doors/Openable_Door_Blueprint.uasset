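; Openable door Actor Blueprint that the player swings open and shut with the E key while near it.
; A Box trigger enables player 0's input on any begin overlap and disables it on end overlap, without checking the overlapping actor.
; E plays or reverses the DoorRotation timeline, which drives the Door's relative yaw.
; Tick derives IsClosed from the timeline value, counting the door closed only near zero rotation.
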(event OnComponentBeginOverlap(Box)
  (params (OverlappedComponent :type Primitive%20Component%20Object%20Reference) (OtherActor :type Actor%20Object%20Reference) (OtherComp :type Primitive%20Component%20Object%20Reference) (OtherBodyIndex :type Integer) (bFromSweep :type Boolean) (SweepResult :type Hit%20Result%20Structure%20%28by%20ref%29))
  ;[1 1 1] Check Player is in range to give an Input
  (Input|EnableInput (Game|GetPlayerController 0)))

(event OnComponentEndOverlap(Box)
  (params (OverlappedComponent :type Primitive%20Component%20Object%20Reference) (OtherActor :type Actor%20Object%20Reference) (OtherComp :type Primitive%20Component%20Object%20Reference) (OtherBodyIndex :type Integer))
  ;[1 1 1] Check Player is in range to give an Input
  (Input|DisableInput (Game|GetPlayerController 0)))

(event EventTick
  (params (DeltaSeconds :type Float%20%28single-precision%29))
  ;[1 1 1] If in range to receive an input, open/close Door
  (Variables|Default|SetIsClosed (< (stale Input|KeyboardEvents|E _doorrot) 1.0)))

(event Input|KeyboardEvents|E
  (params (Key :type Key%20Structure :default "AnyKey"))
  ;[1 1 1] If in range to receive an input, open/close Door
  (:Pressed
    (if (Variables|Default|GetIsClosed)
      (bind _doorrot (Timeline|Door%20Rotation Play)
        (:Update
          (Transformation|SetRelativeRotation (Variables|Default|GetDoor) (Math|Rotator|MakeRotator 0.0 0.0 _doorrot) false false)))
      (else
        (Timeline|Door%20Rotation Reverse)))))

(fn ConstructionScript)